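; BP_CheckPoint is an overlap-triggered checkpoint actor that records the player's progress.
; When the overlapping actor matches the stored player reference, it saves the player's HP and score to the game instance, along with itself as the last checkpoint.
; A DoOnce gate with no reset wired limits each checkpoint to a single save.
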(event `self.ReceiveActorBeginOverlap`
  (params (OtherActor :type "Actor Object Reference"))
  (if (== OtherActor (`self.AsPlayer`))
    (`/Engine/EditorBlueprintResources/StandardMacros.DoOnce` false
      (:`Completed`
        (set `/Game/Blueprints/Config/BP_MyGameInstance.LastHP` (`/Game/ThirdPerson/Blueprints/BP_ThirdPersonCharacter.HP` (`self.AsPlayer`)) (`self.AsGameInstance`))
        (set `/Game/Blueprints/Config/BP_MyGameInstance.LastScore` (`/Game/ThirdPerson/Blueprints/BP_ThirdPersonCharacter.Score` (`self.AsPlayer`)) (`self.AsGameInstance`))
        (set `/Game/Blueprints/Config/BP_MyGameInstance.LastCheckpoint` (`|ConvertAsset` self) (`self.AsGameInstance`))))))

(fn `UserConstructionScript`)