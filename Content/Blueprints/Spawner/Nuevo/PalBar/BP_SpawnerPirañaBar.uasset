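; Spawner actor that places piranha AI with their behavior tree at random points inside a box when the player comes within range.
; Tick checks the distance, then spawns the batch once and disables itself; the looping timer it sets targets an empty event.
; RevisarEnemigos prunes invalid entries and refills Enemigos to five, but nothing here calls it, and the initial batch is never added to that array.
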(event `self.ReceiveTick`
  (params (DeltaSeconds :type "Float (single-precision)"))
  (bind _returnvalue (`KismetSystemLibrary.K2_SetTimerDelegate` (delegate `checkplayerrange`) 0.2 true))
  (if (and (<= (`KismetMathLibrary.Vector_Distance` (`self.K2_GetActorLocation` (`GameplayStatics.GetPlayerCharacter` 0)) (`self.K2_GetActorLocation`)) (`self.SpawnRange`)) (== (`self.bSpawnerActivo`) false))
    (`KismetSystemLibrary.K2_ClearAndInvalidateTimerHandle` _returnvalue)
    (`self.SpawnEnemigos`)))

(event `checkplayerrange`)

(event `SpawnEnemigos`
  (bind (_origin _boxextent) (`KismetSystemLibrary.GetComponentBounds` (`self.Box`)))
  (if (not (`self.bSpawnerActivo`))
    (for _ (range (`self.MaxSpawns`))
      (`AIBlueprintHelperLibrary.SpawnAIFromClass` "/Game/Blueprints/IA/Piraña/AI_Piraña.AI_Piraña_C" "/Game/Blueprints/IA/Piraña/BT_Piraña.BT_Piraña" (`KismetMathLibrary.RandomPointInBoundingBox` _origin _boxextent) (struct) false null)
      (`self.SetActorTickEnabled` false))
    (set `self.bSpawnerActivo` true)))

(event `RevisarEnemigos`
  (bind (_arrayindex _arrayelement) (`/Engine/EditorBlueprintResources/StandardMacros.ReverseForEachLoop` (`self.Enemigos`))
    (:`LoopBody`
      (`/Engine/EditorBlueprintResources/StandardMacros.IsValid` _arrayelement
        (:`Is Not Valid`
          (`KismetArrayLibrary.Array_Remove` (`self.Enemigos`) _arrayindex))))
    (:`Completed`
      (`self.RespawnEnemigos`))))

(event `RespawnEnemigos`
  (bind _returnvalue (`KismetArrayLibrary.Array_Length` (`self.Enemigos`)))
  (bind (_origin _boxextent) (`KismetSystemLibrary.GetComponentBounds` (`self.Box`)))
  (if (< _returnvalue 5)
    (for _ (range 1 (+ (- 5 _returnvalue) 1))
      (bind _returnvalue_2 (`AIBlueprintHelperLibrary.SpawnAIFromClass` "/Game/Blueprints/IA/Piraña/AI_Piraña.AI_Piraña_C" "/Game/Blueprints/IA/Piraña/BT_Piraña.BT_Piraña" (`KismetMathLibrary.RandomPointInBoundingBox` _origin _boxextent) (struct) false null))
      (`KismetArrayLibrary.Array_Add` (`self.Enemigos`) _returnvalue_2))))

(fn `UserConstructionScript`)