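; Spawner that keeps a population of five piranha AI enemies inside a box volume.
; A looping timer started on BeginPlay frequently prunes invalid entries from the Enemigos array, iterating in reverse so removal is safe.
; It then spawns any missing piranhas with their behavior tree at random points within the Box bounds and adds them to the array.
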(event `self.ReceiveBeginPlay`
  (`KismetSystemLibrary.K2_SetTimerDelegate` (delegate `RevisarEnemigos`) 0.1 true))

(event `RevisarEnemigos`
  (bind (_arrayindex _arrayelement) (`/Engine/EditorBlueprintResources/StandardMacros.ReverseForEachLoop` (`self.Enemigos`))
    (:`LoopBody`
      (`/Engine/EditorBlueprintResources/StandardMacros.IsValid` _arrayelement
        (:`Is Not Valid`
          (`KismetArrayLibrary.Array_Remove` (`self.Enemigos`) _arrayindex))))
    (:`Completed`
      (`self.RespawnEnemigos`))))

(event `RespawnEnemigos`
  (bind _returnvalue (`KismetArrayLibrary.Array_Length` (`self.Enemigos`)))
  (bind (_origin _boxextent) (`KismetSystemLibrary.GetComponentBounds` (`self.Box`)))
  (if (< _returnvalue 5)
    (for _ (range 1 (+ (- 5 _returnvalue) 1))
      (bind _returnvalue_2 (`AIBlueprintHelperLibrary.SpawnAIFromClass` "/Game/Blueprints/IA/Piraña/AI_Piraña.AI_Piraña_C" "/Game/Blueprints/IA/Piraña/BT_Piraña.BT_Piraña" (`KismetMathLibrary.RandomPointInBoundingBox` _origin _boxextent) (struct) false null))
      (`KismetArrayLibrary.Array_Add` (`self.Enemigos`) _returnvalue_2))))

(fn `UserConstructionScript`)