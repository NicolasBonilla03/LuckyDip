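; FL_HPScore is a function library that changes a player's HP and score.
; AddHP zeroes HP and calls CEDie on lethal changes, otherwise applies gains directly with no upper cap.
; Non-lethal damage calls TakeDamage and prints HP when Bcantakedamage is false; when true, only poisoned players lose HP, without that call.
; AddScore adds to Score, flooring it at zero.
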(fn `AddHP`
  (params (HpToAdd1 :type Integer) (Player1 :type "/Game/ThirdPerson/Blueprints/BP_ThirdPersonCharacter Object Reference"))
  (locals (HpToAdd :type Integer) (Player :type "/Game/ThirdPerson/Blueprints/BP_ThirdPersonCharacter Object Reference") (IsInvunerable :type Boolean :default false))
  (bind _player (`local.Player`))
  (bind _player_2 (`local.Player`))
  (bind _player_3 (`local.Player`))
  (set `local.HpToAdd` HpToAdd1)
  (bind _output_get (set `local.Player` Player1))
  (if (`KismetSystemLibrary.IsValid` _output_get)
    (if (<= (+ (`/Game/ThirdPerson/Blueprints/BP_ThirdPersonCharacter.HP` (`local.Player`)) (`local.HpToAdd`)) 0)
      (`/Engine/EditorBlueprintResources/StandardMacros.IsValid` _player_3
        (:`Is Valid`
          (set `/Game/ThirdPerson/Blueprints/BP_ThirdPersonCharacter.HP` 0 _player_3)
          (`/Game/ThirdPerson/Blueprints/BP_ThirdPersonCharacter.CE_Die` (`local.Player`))
          (return)))
      (elif (>= (+ (`/Game/ThirdPerson/Blueprints/BP_ThirdPersonCharacter.HP` (`local.Player`)) (`local.HpToAdd`)) (`/Game/ThirdPerson/Blueprints/BP_ThirdPersonCharacter.HP` (`local.Player`)))
        (set `/Game/ThirdPerson/Blueprints/BP_ThirdPersonCharacter.HP` (+ (`local.HpToAdd`) (`/Game/ThirdPerson/Blueprints/BP_ThirdPersonCharacter.HP` _player)) _player)
        (return)
        (else
          (if (> (`local.HpToAdd`) 0)
            (set `/Game/ThirdPerson/Blueprints/BP_ThirdPersonCharacter.HP` (`local.HpToAdd`) (`local.Player`)))
          (if (`/Game/ThirdPerson/Blueprints/BP_ThirdPersonCharacter.bcantakedamage` (`local.Player`))
            (if (`/Game/ThirdPerson/Blueprints/BP_ThirdPersonCharacter.isPoisoned` _player_2)
              (bind _output_get_2 (set `/Game/ThirdPerson/Blueprints/BP_ThirdPersonCharacter.HP` (+ (`/Game/ThirdPerson/Blueprints/BP_ThirdPersonCharacter.HP` (`local.Player`)) (`local.HpToAdd`)) (`local.Player`) :!label _label))
              (`KismetSystemLibrary.PrintString` null (`KismetStringLibrary.Conv_IntToString` _output_get_2))
              (return))
            (else
              (`/Game/ThirdPerson/Blueprints/BP_ThirdPersonCharacter.TakeDamage` _player_2)
              (goto _label))))))))

(fn `AddScore`
  (params (ScoreToAdd1 :type Integer) (Player1 :type "/Game/ThirdPerson/Blueprints/BP_ThirdPersonCharacter Object Reference"))
  (locals (Player :type "/Game/ThirdPerson/Blueprints/BP_ThirdPersonCharacter Object Reference") (ScoreToAdd :type Integer))
  (set `local.ScoreToAdd` ScoreToAdd1)
  (set `local.Player` Player1)
  (if (<= (+ (`local.ScoreToAdd`) (`/Game/ThirdPerson/Blueprints/BP_ThirdPersonCharacter.Score` (`local.Player`))) 0)
    (set `/Game/ThirdPerson/Blueprints/BP_ThirdPersonCharacter.Score` 0 (`local.Player`))
    (else
      (set `/Game/ThirdPerson/Blueprints/BP_ThirdPersonCharacter.Score` (+ (`local.ScoreToAdd`) (`/Game/ThirdPerson/Blueprints/BP_ThirdPersonCharacter.Score` (`local.Player`))) (`local.Player`))))
  (return))