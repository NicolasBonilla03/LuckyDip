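; BP_Item is an interactive item actor that toggles between attached to the player and released on the grab input.
; When IA_Grab starts, the IsAttached flag decides whether it snaps to a socket on the player's mesh, named by Player.SocketName3, or detaches keeping its world position and rotation.
; The graph makes no range, overlap or validity check before attaching.
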(event `EnhancedInput|/Game/ThirdPerson/Input/Actions/IA_Grab`
  (params (ActionValue :type Boolean) (ElapsedSeconds :type "Float (double-precision)") (TriggeredSeconds :type "Float (double-precision)") (InputAction :type "InputAction Object Reference" :default "/Game/ThirdPerson/Input/Actions/IA_Grab.IA_Grab"))
  (:`Started`
    (if (`self.isAttached`)
      (`self.K2_DetachFromActor` self "KeepWorld" "KeepWorld" "KeepRelative")
      (set `self.isAttached` false)
      (else
        (`self.K2_AttachToComponent` self (`Character.Mesh` (`self.Player`)) (`/Game/ThirdPerson/Blueprints/BP_ThirdPersonCharacter.SocketName3` (`self.Player`)) "SnapToTarget" "SnapToTarget" "KeepRelative" false)
        (set `self.isAttached` true)))))

(fn `UserConstructionScript`)