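; BP_DoorKeyEnd is a key actor the player picks up and drops to unlock and relock its linked door.
; The Interact input toggles it, with no range check in this graph, between snapping to the character mesh's LlaveSocket and detaching in place.
; Pickup unlocks MyDoor and hides the sprite; dropping relocks the door but leaves the sprite hidden.
; The construction script applies an override mesh to the key.
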(event `EnhancedInput|/Game/ThirdPerson/Input/Actions/IA_Interact`
  (params (ActionValue :type Boolean) (ElapsedSeconds :type "Float (double-precision)") (TriggeredSeconds :type "Float (double-precision)") (InputAction :type "InputAction Object Reference" :default "/Game/ThirdPerson/Input/Actions/IA_Interact.IA_Interact"))
  (bind _mydoor (`self.MyDoor`))
  (bind _mydoor_2 (`self.MyDoor`))
  (:`Started`
    (if (`self.IsAttached`)
      (`self.K2_DetachFromActor` self "KeepWorld" "KeepWorld" "KeepWorld")
      (set `self.IsAttached` false)
      (`/Engine/EditorBlueprintResources/StandardMacros.IsValid` _mydoor
        (:`Is Valid`
          (set `/Game/Blueprints/OverlappingActors/BP_DoorEnd.IsLocked` true _mydoor)))
      (else
        (bind _asbp_third_person_character (cast `/Game/ThirdPerson/Blueprints/BP_ThirdPersonCharacter` (`GameplayStatics.GetPlayerCharacter` 0)))
        (`self.K2_AttachToComponent` self (`Character.Mesh` _asbp_third_person_character) "LlaveSocket" "SnapToTarget" "SnapToTarget" "KeepWorld" false)
        (set `self.IsAttached` true)
        (`SceneComponent.SetVisibility` (`self.Sprite`) false false)
        (`/Engine/EditorBlueprintResources/StandardMacros.IsValid` _mydoor_2
          (:`Is Valid`
            (set `/Game/Blueprints/OverlappingActors/BP_DoorEnd.IsLocked` false _mydoor_2)))))))

(fn `UserConstructionScript`
  (`StaticMeshComponent.SetStaticMesh` (`self.KeyMesh`) (`self.KeyMeshOverRide`)))